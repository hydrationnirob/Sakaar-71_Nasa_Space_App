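; Checkpoint actor for the Mars rover that serves as the compass nav target and reacts to overlap.
; It caches the player's BP_Vehicle on BeginPlay and writes its own location to the vehicle's NavPoint every Tick.
; Box overlap, with no check on the entering actor, sets the vehicle's CheckpointOverlap flag, plays a sound and scales the checkpoint up through a timeline.
; Leaving clears the flag and reverses the timeline.
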(event `self.ReceiveBeginPlay`
  ;[1 1 1] Cast To BP_Vehicle
  (bind _asbp_vehicle (cast `/Game/MarsRover/Blueprints/Rover/BP_Vehicle` (`GameplayStatics.GetPlayerPawn` 0)))
  (bind _output_get (set `self.BP_MarsRover_Ref` _asbp_vehicle)))

(event `self.ReceiveTick`
  (params (DeltaSeconds :type "Float (single-precision)"))
  ;[1 1 1] For Marker Of Compass
  (set `/Game/MarsRover/Blueprints/Rover/BP_Vehicle.Nav Point` (`self.K2_GetActorLocation`) (stale `self.ReceiveBeginPlay` _output_get)))

(event `self.Box.OnComponentBeginOverlap`
  (params (OverlappedComponent :type "PrimitiveComponent Object Reference") (OtherActor :type "Actor Object Reference") (OtherComp :type "PrimitiveComponent Object Reference") (OtherBodyIndex :type Integer) (bFromSweep :type Boolean) (SweepResult :type "HitResult Structure (by ref)"))
  ;[1 1 1] Checkpoint Overlap
  (set `/Game/MarsRover/Blueprints/Rover/BP_Vehicle.CheckpointOverlap?` true (`self.BP_MarsRover_Ref`))
  (`GameplayStatics.PlaySound2D` "/Game/MarsRover/SoundEffect/S_CheckpointOverlap_Cue.S_CheckpointOverlap_Cue" 1.0 1.0 0.0 null null)
  (bind (_direction _scalcheckpoint) (`Timeline|CheckpointLerp` :!label _label)
    (:`Update`
      (`self.SetActorScale3D` (`KismetMathLibrary.VLerp` (0.6 0.6 0.6) (1.1 1.1 1.1) _scalcheckpoint)))))

(event `self.Box.OnComponentEndOverlap`
  (params (OverlappedComponent :type "PrimitiveComponent Object Reference") (OtherActor :type "Actor Object Reference") (OtherComp :type "PrimitiveComponent Object Reference") (OtherBodyIndex :type Integer))
  ;[1 1 1] Checkpoint Overlap
  (set `/Game/MarsRover/Blueprints/Rover/BP_Vehicle.CheckpointOverlap?` false (`self.BP_MarsRover_Ref`))
  (goto _label :!via `Reverse`))

(fn `UserConstructionScript`)